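; BP_HealthPack is a timed health pickup that destroys itself seven seconds after it spawns.
; When a BP_Player overlaps its Health_Pack component and has nonzero health, it adds a fixed amount of health, clamped to the maximum, then destroys itself.
; Player projectiles that hit it are destroyed with a debug print, leaving the pack intact.
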(event OnComponentBeginOverlap(Health_Pack)
  (params (OverlappedComponent :type Primitive%20Component%20Object%20Reference) (OtherActor :type Actor%20Object%20Reference) (OtherComp :type Primitive%20Component%20Object%20Reference) (OtherBodyIndex :type Integer) (bFromSweep :type Boolean) (SweepResult :type Hit%20Result%20Structure%20%28by%20ref%29))
  (bind _asbp_player (Utilities|Casting|CastToBP_Player OtherActor)
    (:then
      (if (not (== (Variables|/Game/InfiniteMatrix/Blueprints/BP_Player.BP_Player_C|GetHealth _asbp_player) 0.0))
        (Variables|/Game/InfiniteMatrix/Blueprints/BP_Player.BP_Player_C|SetHealth _asbp_player (Math|Float|Clamp(Float) (+ (Variables|/Game/InfiniteMatrix/Blueprints/BP_Player.BP_Player_C|GetHealth _asbp_player) 1e+01) 0.0 1e+02))
        (Actor|DestroyActor)))
    (:CastFailed
      (bind _asbp_player_projectile (Utilities|Casting|CastToBP_Player_Projectile OtherActor))
      (Actor|DestroyActor _asbp_player_projectile)
      (Development|PrintString "Bullet hit HealthPack"))))

(event Collision|EventActorBeginOverlap
  (params (OtherActor :type Actor%20Object%20Reference)))

(event EventBeginPlay
  (Utilities|FlowControl|Delay 7.0)
  (Actor|DestroyActor))

(fn ConstructionScript)