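; BP_Enemy is an enemy actor that damages the player on contact and removes itself seven seconds after spawning.
; Overlap on its ROBOT component subtracts clamped health from BP_Player, destroys the enemy, and calls DisplayRestart on the player when health reaches zero.
; Other actors are cast to BP_Player_Projectile, but the logic to destroy both projectile and enemy is disconnected and never runs.
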(event OnComponentBeginOverlap(ROBOT)
  (params (OverlappedComponent :type Primitive%20Component%20Object%20Reference) (OtherActor :type Actor%20Object%20Reference) (OtherComp :type Primitive%20Component%20Object%20Reference) (OtherBodyIndex :type Integer) (bFromSweep :type Boolean) (SweepResult :type Hit%20Result%20Structure%20%28by%20ref%29))
  (bind _asbp_player (Utilities|Casting|CastToBP_Player OtherActor)
    (:then
      (Variables|/Game/InfiniteMatrix/Blueprints/BP_Player.BP_Player_C|SetHealth _asbp_player (Math|Float|Clamp(Float) (- (Variables|/Game/InfiniteMatrix/Blueprints/BP_Player.BP_Player_C|GetHealth _asbp_player) 25.0) 0.0 1e+02))
      (Actor|DestroyActor)
      (if (== (Variables|/Game/InfiniteMatrix/Blueprints/BP_Player.BP_Player_C|GetHealth _asbp_player) 0.0)
        (Default|DisplayRestart _asbp_player)))
    (:CastFailed
      (bind _asbp_player_projectile (Utilities|Casting|CastToBP_Player_Projectile OtherActor)))))

(event Collision|EventActorBeginOverlap
  (params (OtherActor :type Actor%20Object%20Reference)))

(event EventTick
  (params (DeltaSeconds :type Float%20%28single-precision%29)))

(event EventBeginPlay
  (Utilities|FlowControl|Delay 7.0)
  (Actor|DestroyActor))

(fn ConstructionScript)